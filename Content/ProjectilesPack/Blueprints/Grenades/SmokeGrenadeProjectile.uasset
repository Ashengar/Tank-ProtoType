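; Smoke grenade projectile that detonates on collision, after an optional travel distance, or after an optional fuse time.
; BeginPlay records the start location and runs the timer, while Tick checks distance travelled.
; All triggers share a DoOnce explosion that fires a radial impulse, executes the smoke payload and tells the child grenade actor to destroy itself.
; Radial damage reuses the radial force component's radius and destructible damage.
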(event `self.ReceiveTick`
  (params (DeltaSeconds :type "Float (single-precision)"))
  ;[1 1 1] Explode after specified amount of distance
  (if (`self.UseExplodeDistance`)
    (if (>= (`KismetMathLibrary.VSize` (- (`SceneComponent.K2_GetComponentLocation` (`self.CollisionComponent`)) (`self.StartLocation`))) (`self.ExplodeDistance`))
      (`self.Explode`))))

(event `self.ReceiveBeginPlay`
  ;[1 1 1] Get start location
  (set `self.StartLocation` (`SceneComponent.K2_GetComponentLocation` (`self.CollisionComponent`)))
  ;[1 1 1] Explode after specified amount of time
  (if (`self.UseExplodeTime`)
    (`KismetSystemLibrary.Delay` (`self.ExplodeTime`))
    (`self.Explode`)))

(event `Explode`
  (bind _explosionforce (`self.ExplosionForce`))
  ;[1 1 1] On hit or explode event
  (`/Engine/EditorBlueprintResources/StandardMacros.DoOnce` false :!label _label
    (:`Completed`
      ;[1 1 1] Fire impulse
      (`RadialForceComponent.FireImpulse` (`self.ExplosionForce`))
      ;[1 1 1] Execute payload
      (`/Game/ProjectilesPack/Blueprints/Payloads/SmokePayload.Execute` (`self.SmokePayload`) (`SceneComponent.K2_GetComponentLocation` (`self.ExplosionForce`)))
      ;[1 1 1] Destroy grenade
      (message `/Game/ProjectilesPack/Blueprints/Common/AdvancedProjectile.Destroy` (`ChildActorComponent.ChildActor` (`self.BP_Grenade`)))
      ;[1 1 1] Apply damage
      (`GameplayStatics.ApplyRadialDamage` :`BaseDamage` (`RadialForceComponent.DestructibleDamage` _explosionforce) :`Origin` (`SceneComponent.K2_GetComponentLocation` _explosionforce) :`DamageRadius` (`RadialForceComponent.Radius` _explosionforce) :`DamageTypeClass` "/Script/Engine.DamageType" :`DamageCauser` self))))

(event `self.CollisionComponent.OnComponentHit`
  (params (OtherActor :type "Actor Object Reference") (OtherComp :type "PrimitiveComponent Object Reference") (NormalImpulse :type "Vector Structure") (Hit :type "HitResult Structure (by ref)"))
  ;[1 1 1] On hit or explode event
  (goto _label))

(fn `UserConstructionScript`)