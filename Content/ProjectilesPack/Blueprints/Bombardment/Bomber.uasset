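; Bomber aircraft actor for a bombardment, which flies in fast, drops bombs and speeds away.
; On BeginPlay, the SpeedDown timeline slows its projectile movement component along the X axis.
; It then spawns scaled-up bomb projectile pairs left and right below the bomber at a set interval, using a delayed loop until the count reaches BombsCount.
; After a short delay, the SpeedUp timeline accelerates it again.
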(event `self.ReceiveBeginPlay`
  ;[1 1 1] Decrease bomber speed after spawn
  (bind (_direction _speed) (`Timeline|SpeedDown` :!via `PlayFromStart`)
    (:`Update`
      (bind _returnvalue (`KismetMathLibrary.Lerp` 30000.0 5000.0 _speed))
      (set `ProjectileMovementComponent.MaxSpeed` _returnvalue (`self.Projectile`))
      (set `MovementComponent.Velocity` (`KismetMathLibrary.MakeVector` _returnvalue) (`self.Projectile`)))
    (:`Finished`
      (set `ProjectileMovementComponent.MaxSpeed` 20000.0 (`self.Projectile`))
      (set `MovementComponent.Velocity` (5000.0 0.0 0.0) (`self.Projectile`))
      ;[1 1 1] Repeat until all bombs won't be spawned
      (if (< (`self.SpawnedBombsCount`) (`self.BombsCount`)) :!label _label
        ;[1 1 1] Increment bombs count
        (`/Engine/EditorBlueprintResources/StandardMacros.IncrementInt` (`self.SpawnedBombsCount`)
          (:`  `
            ;[1 1 1] Spawn left bomb
            (bind _returnvalue_2 (`|SpawnActorFromClass` "/Game/ProjectilesPack/Blueprints/Bombardment/BombProjectile.BombProjectile_C" (`KismetMathLibrary.MakeTransform` (+ (`SceneComponent.K2_GetComponentLocation` (`self.Bomber`)) (0.0 100.0 -500.0)) (struct)) "Undefined" "OverrideRootScale"))
            (`self.SetActorScale3D` _returnvalue_2 (5.0 5.0 5.0))
            ;[1 1 1] Spawn right bomb
            (bind _returnvalue_3 (`|SpawnActorFromClass` "/Game/ProjectilesPack/Blueprints/Bombardment/BombProjectile.BombProjectile_C" (`KismetMathLibrary.MakeTransform` (+ (`SceneComponent.K2_GetComponentLocation` (`self.Bomber`)) (0.0 -100.0 -500.0))) "Undefined" "OverrideRootScale"))
            (`self.SetActorScale3D` _returnvalue_3 (5.0 5.0 5.0))
            ;[1 1 1] Delay before next bomb
            (`KismetSystemLibrary.Delay` (`self.BombSpawnInterval`))
            (goto _label)))
        (else
          ;[1 1 1] Increase bomber's speed after bombardment
          (`KismetSystemLibrary.Delay` 3.0)
          (bind (_direction_2 _speed_2) (`Timeline|SpeedUp` :!via `PlayFromStart`)
            (:`Update`
              (set `MovementComponent.Velocity` (`KismetMathLibrary.MakeVector` (`KismetMathLibrary.Lerp` (.x (`MovementComponent.Velocity` (`self.Projectile`))) 20000.0 _speed_2)) (`self.Projectile`)))))))))

(fn `UserConstructionScript`)